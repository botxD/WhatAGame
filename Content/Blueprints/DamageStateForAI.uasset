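; Anim notify state that opens and closes an enemy's sword damage window during an animation.
; On begin and end, it casts the mesh owner to EnemyBlueprint and its child actor to BaseSwordClass.
; It calls SwordActive when the window starts and SwordDeactive when it ends, doing nothing if either cast fails.
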(fn ReceivedNotifyBegin
  (params (MeshComp :type Skeletal%20Mesh%20Component%20Object%20Reference) (Animation :type Anim%20Sequence%20Base%20Object%20Reference) (TotalDuration :type Float%20%28single-precision%29))
  (bind _asenemy_blueprint (Utilities|Casting|CastToEnemyBlueprint (Components|GetOwner MeshComp)))
  (bind _asbase_sword_class (Utilities|Casting|CastToBaseSwordClass (Variables|/Script/Engine.ChildActorComponent|GetChildActor (Variables|/Game/TrueAI/EnemyBlueprint.EnemyBlueprint_C|GetChildActor _asenemy_blueprint))))
  (Default|SwordActive _asbase_sword_class)
  (return false))

(fn ReceivedNotifyEnd
  (params (MeshComp :type Skeletal%20Mesh%20Component%20Object%20Reference) (Animation :type Anim%20Sequence%20Base%20Object%20Reference))
  (bind _asenemy_blueprint (Utilities|Casting|CastToEnemyBlueprint (Components|GetOwner MeshComp)))
  (bind _asbase_sword_class (Utilities|Casting|CastToBaseSwordClass (Variables|/Script/Engine.ChildActorComponent|GetChildActor (Variables|/Game/TrueAI/EnemyBlueprint.EnemyBlueprint_C|GetChildActor _asenemy_blueprint))))
  (Default|SwordDeactive _asbase_sword_class)
  (return false))