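; DamageState is an animation notify state that opens and closes the player's sword damage window during an animation.
; On begin and end it casts the mesh owner to PlayerBlueprint and its child actor to BaseSwordClass.
; It then calls SwordActive at the start and SwordDeactive at the end, leaving the hit logic to the sword.
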(fn ReceivedNotifyBegin
  (params (MeshComp :type Skeletal%20Mesh%20Component%20Object%20Reference) (Animation :type Anim%20Sequence%20Base%20Object%20Reference) (TotalDuration :type Float%20%28single-precision%29))
  (bind _asplayer_blueprint (Utilities|Casting|CastToPlayerBlueprint (Components|GetOwner MeshComp)))
  (bind _asbase_sword_class (Utilities|Casting|CastToBaseSwordClass (Variables|/Script/Engine.ChildActorComponent|GetChildActor (Variables|/Game/PlayerFolder/PlayerBlueprint.PlayerBlueprint_C|GetChildActor _asplayer_blueprint))))
  (Default|SwordActive _asbase_sword_class)
  (return false))

(fn ReceivedNotifyEnd
  (params (MeshComp :type Skeletal%20Mesh%20Component%20Object%20Reference) (Animation :type Anim%20Sequence%20Base%20Object%20Reference))
  (bind _asplayer_blueprint (Utilities|Casting|CastToPlayerBlueprint (Components|GetOwner MeshComp)))
  (bind _asbase_sword_class (Utilities|Casting|CastToBaseSwordClass (Variables|/Script/Engine.ChildActorComponent|GetChildActor (Variables|/Game/PlayerFolder/PlayerBlueprint.PlayerBlueprint_C|GetChildActor _asplayer_blueprint))))
  (Default|SwordDeactive _asbase_sword_class)
  (return false))