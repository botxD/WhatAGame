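; BP_SpawnPoint is a spawner that populates a bounded area with AI enemies and keeps their count topped up.
; On BeginPlay it spawns SpawnAmount enemies, then a looping timer adds one whenever ActivePawns falls below that amount.
; Each spawn traces down against WorldStatic from high above a random point in Bound to find ground.
; Spawned enemies get a default controller and a reference back to the spawn point.
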(event EventBeginPlay
  (for _index (range 1 (Variables|Default|GetSpawnAmount))
    (CallFunction|SpawnCharacter))
  (Utilities|Time|SetTimerbyFunctionName 0 "RespawnCharacter" (Variables|Default|GetTimeToRespawn) true))

(fn ConstructionScript)

(fn SpawnCharacter
  (bind _bound (Variables|Default|GetBound))
  (bind (_origin _boxextent) (Collision|GetComponentBounds _bound))
  (bind _returnvalue (Math|Random|RandomPointinBoundingBox _origin _boxextent))
  (bind (_x _y _z) (Math|Vector|BreakVector _returnvalue))
  (bind _returnvalue_2 (+ _z 1e+04))
  (bind _returnvalue_3 (Math|Vector|MakeVector _x _y _returnvalue_2))
  (bind _outhit (Collision|LineTraceForObjects _returnvalue_3 (+ _returnvalue_3 (* (* (Transformation|GetActorUpVector) -1.0) 1.5e+04)) (Utilities|Array|MakeArray "ObjectTypeQuery1") false 0 "ForDuration"))
  (bind _returnvalue_4 (Game|SpawnActorfromClass "/Game/TrueAI/EnemyBlueprint.EnemyBlueprint_C" (Math|Transform|MakeTransform (Math|Vector|MakeVector (.X (Math|Vector|BreakVector (.ImpactPoint (Collision|BreakHitResult _outhit)))) (.Y (Math|Vector|BreakVector (.ImpactPoint (Collision|BreakHitResult _outhit)))) (+ (.Z (Math|Vector|BreakVector (.ImpactPoint (Collision|BreakHitResult _outhit)))) 1e+02)) (Math|Rotator|MakeRotator 0.0 0.0 (Math|Random|RandomFloat))) "AdjustIfPossibleButAlwaysSpawn" 0 0))
  (Pawn|SpawnDefaultController _returnvalue_4)
  (Variables|/Game/TrueAI/EnemyBlueprint.EnemyBlueprint_C|SetSpawnPoint _returnvalue_4 self)
  (Utilities|Array|Add (Variables|Default|GetActivePawns) _returnvalue_4))

(fn RespawnCharacter
  (if (< (Utilities|Array|Length (Variables|Default|GetActivePawns)) (Variables|Default|GetSpawnAmount))
    (CallFunction|SpawnCharacter)))